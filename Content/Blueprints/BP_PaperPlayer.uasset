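; BP_PaperPlayer is a Paper2D player character Blueprint that switches sprite flipbook animations on jump and landing.
; OnJumped starts looping playback with no flipbook specified, while OnLanded plays the landing flipbook once and binds the sprite's finished-playing event to return to the looping run cycle.
; A shared PlayAnimation helper sets the flipbook and looping flag, then plays the sprite.
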(event `self.OnJumped`
  (`self.PlayAnimation` true))

(event `self.OnLanded`
  (params (Hit :type "HitResult Structure (by ref)"))
  (`self.PlayAnimation` false "/Game/Animations/PlayerLand/PF_PlayerLand01.PF_PlayerLand01")
  (add `PaperFlipbookComponent.OnFinishedPlaying` (`self.Sprite`) (delegate `OnFinishedPlaying_Event`)))

(event `OnFinishedPlaying_Event`
  (`self.PlayAnimation` true "/Game/Animations/PlayerRun/PF_PlayerRunCycle.PF_PlayerRunCycle"))

(fn `PlayAnimation`
  (params (bLoop :type Boolean) (Flipbook :type "PaperFlipbook Object Reference"))
  (bind _sprite (`self.Sprite`))
  (`PaperFlipbookComponent.SetFlipbook` _sprite Flipbook)
  (`PaperFlipbookComponent.SetLooping` _sprite bLoop)
  (`PaperFlipbookComponent.Play` _sprite))

(fn `UserConstructionScript`)